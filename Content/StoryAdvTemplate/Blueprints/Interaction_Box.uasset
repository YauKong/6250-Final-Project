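; Interaction_Box is a trigger volume that shows an interaction prompt when the narrative third-person player character is inside it.
; On Box begin and end overlap, it casts the other actor to BP_ThirdPersonCharacter_Narrative so other actors are ignored.
; It then reaches the interaction UI through Level_GameMode and toggles a text block between visible and hidden.
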(event OnComponentBeginOverlap(Box)
  (params (OverlappedComponent :type Primitive%20Component%20Object%20Reference) (OtherActor :type Actor%20Object%20Reference) (OtherComp :type Primitive%20Component%20Object%20Reference) (OtherBodyIndex :type Integer) (bFromSweep :type Boolean) (SweepResult :type Hit%20Result%20Structure%20%28by%20ref%29))
  (Utilities|Casting|CastToBP_ThirdPersonCharacter_Narrative OtherActor)
  (bind _aslevel_game_mode (Utilities|Casting|CastToLevel_GameMode (Game|GetGameMode)))
  (Variables|/Script/UMG.Widget|SetVisibility (Variables|/Game/StoryAdvTemplate/Blueprints/Interaction_UI.Interaction_UI_C|GetTextBlock_0 (Variables|/Game/StoryAdvTemplate/Blueprints/Level_GameMode.Level_GameMode_C|GetAs%20Interaction_UI _aslevel_game_mode)) "Visible"))

(event OnComponentEndOverlap(Box)
  (params (OverlappedComponent :type Primitive%20Component%20Object%20Reference) (OtherActor :type Actor%20Object%20Reference) (OtherComp :type Primitive%20Component%20Object%20Reference) (OtherBodyIndex :type Integer))
  (Utilities|Casting|CastToBP_ThirdPersonCharacter_Narrative OtherActor)
  (bind _aslevel_game_mode (Utilities|Casting|CastToLevel_GameMode (Game|GetGameMode)))
  (Variables|/Script/UMG.Widget|SetVisibility (Variables|/Game/StoryAdvTemplate/Blueprints/Interaction_UI.Interaction_UI_C|GetTextBlock_0 (Variables|/Game/StoryAdvTemplate/Blueprints/Level_GameMode.Level_GameMode_C|GetAs%20Interaction_UI _aslevel_game_mode)) "Hidden"))

(event EventBeginPlay)

(event Collision|EventActorBeginOverlap
  (params (OtherActor :type Actor%20Object%20Reference)))

(event EventTick
  (params (DeltaSeconds :type Float%20%28single-precision%29)))

(fn ConstructionScript)